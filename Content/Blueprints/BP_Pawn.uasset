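; BP_Pawn is a player pawn that moves sideways and launches play by spawning a BP_Ball.
; The Move Right axis drives a frame-rate-independent, swept world offset along Y.
; BeginPlay sets game-only input, then calls SpawnBall, which spawns the ball at the Capsule's location regardless of collision.
; SpawnBall stores the ball as PlayingBall and binds an event to its OnDead dispatcher.
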(event `InputAxis|Move Right`
  (params (AxisValue :type "Float (single-precision)"))
  (`self.K2_AddActorWorldOffset` (`KismetMathLibrary.MakeVector` 0.0 (* AxisValue 4000.0 (`GameplayStatics.GetWorldDeltaSeconds`))) true))

(event `self.ReceiveBeginPlay`
  (`|ExecutionSequence`
    (:`then_0`
      (`WidgetBlueprintLibrary.SetInputMode_GameOnly` (`GameplayStatics.GetPlayerController` 0)))
    (:`then_1`
      (`self.SpawnBall`))))

(fn `SpawnBall`
  (bind _returnvalue (`|SpawnActorFromClass` "/Game/Blueprints/BP_Ball.BP_Ball_C" (`KismetMathLibrary.MakeTransform` (`SceneComponent.K2_GetComponentLocation` (`self.Capsule`))) "AlwaysSpawn" "OverrideRootScale" null null))
  (bind _output_get (set `self.PlayingBall` _returnvalue))
  (add `/Game/Blueprints/BP_Ball.OnDead` _output_get (`|CreateDelegate` :!event `SpawnBall`))
  (return))

(fn `UserConstructionScript`)